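; Industrial robot arm actor for the factory, set up differently for the Real and Twin world types reported by the FactoryNetSubsystem.
; In Real it drops the poseable mesh and plays a one-shot left or right animation, chosen by LeftRight, when an AssemblyLineComponent-tagged component enters its box.
; In Twin it removes the animated mesh and trigger, keeping the poseable mesh with the sparks effect reattached to it.
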(event `self.ReceiveBeginPlay`
  (switch `ETwinWorldType` (`FactoryNetSubsystem.GetTwinWorldType` (subsystem `FactoryNetSubsystem`))
    (:`Twin`
      (`ActorComponent.K2_DestroyComponent` (`self.IndustrialRobot`))
      (`ActorComponent.K2_DestroyComponent` (`self.Box`))
      (`SceneComponent.K2_AttachToComponent` (`self.SparksV2`) (`self.PoseableMesh`) "None" "KeepRelative" "KeepRelative" "KeepRelative" true))
    (:`Real`
      (`ActorComponent.K2_DestroyComponent` (`self.PoseableMesh`)))))

(event `self.ReceiveTick`
  (params (DeltaSeconds :type "Float (single-precision)")))

(event `self.Box.OnComponentBeginOverlap`
  (params (OverlappedComponent :type "PrimitiveComponent Object Reference") (OtherActor :type "Actor Object Reference") (OtherComp :type "PrimitiveComponent Object Reference") (OtherBodyIndex :type Integer) (bFromSweep :type Boolean) (SweepResult :type "HitResult Structure (by ref)"))
  (if (>= (`KismetArrayLibrary.Array_Find` (`ActorComponent.ComponentTags` OtherComp) "AssemblyLineComponent") 0)
    (`SkeletalMeshComponent.PlayAnimation` (`self.IndustrialRobot`) (select `bool` (`self.Left\\Right`) :`false` "/Game/Meshes/RobotLarge/SK_IndustrialRobot_Left_Anim.SK_IndustrialRobot_Left_Anim" :`true` "/Game/Meshes/RobotLarge/SK_IndustrialRobot_Right_Anim.SK_IndustrialRobot_Right_Anim" :!type "AnimationAsset Object Reference") false)))

(fn `UserConstructionScript`)