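; BP_SplineMovable moves a cargo cart front mesh along a spline in a continuous loop.
; On Tick, only while FactoryPosNet's TwinWorldType is Real, it advances a distance by Speed times delta time and resets it to zero at the spline's end.
; The mesh takes the world transform at that distance, without sweep or scale.
; A physics-simulation call is present but never runs.
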(event `self.ReceiveBeginPlay`)

(event `self.ReceiveTick`
  (params (DeltaSeconds :type "Float (single-precision)"))
  (if (`|EnumEquality` (`FactoryNetComponent.TwinWorldType` (`self.FactoryPosNet`)) "Real")
    (bind _output_get (set `self.Pos` (+ (* DeltaSeconds (`self.Speed`)) (`self.Pos`))))
    (if (not (not (>= _output_get (`SplineComponent.GetSplineLength` (`self.Spline`)))))
      (set `self.Pos` 0.0))
    (`SceneComponent.K2_SetWorldTransform` (`self.SM_CargoCart_front`) (`SplineComponent.GetTransformAtDistanceAlongSpline` (`self.Spline`) (`self.Pos`) "World" false) false false)))

(fn `UserConstructionScript`)