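; Pawn for the Cesium factory editor that flies the view to locations on the globe.
; FlyToEarthView sends its FlyTo component to a given globe anchor's longitude, latitude and height, using that anchor's east-south-up rotation for yaw and pitch.
; FlyToOrigin flies to the origin of its own GlobeAnchor's georeference.
; The event graph holds only disabled default events.
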(fn `FlyToEarthView`
  (params (InGlobeAnchor :type "CesiumGlobeAnchorComponent Object Reference"))
  (bind (_returnvalue_roll _returnvalue_pitch _returnvalue_yaw) (`KismetMathLibrary.BreakRotator` (`KismetMathLibrary.Quat_Rotator` (`CesiumGlobeAnchorComponent.GetEastSouthUpRotation` InGlobeAnchor))))
  (`CesiumFlyToComponent.FlyToLocationLongitudeLatitudeHeight` (`self.FlyTo`) (`CesiumGlobeAnchorComponent.GetLongitudeLatitudeHeight` InGlobeAnchor) _returnvalue_yaw _returnvalue_pitch false))

(fn `FlyToOrigin`
  (`CesiumFlyToComponent.FlyToLocationLongitudeLatitudeHeight` (`self.FlyTo`) (`CesiumGeoreference.GetOriginLongitudeLatitudeHeight` (`|ConvertAsset` (`CesiumGlobeAnchorComponent.Georeference` (`self.GlobeAnchor`)))) 0.0 0.0 false))

(fn `UserConstructionScript`
  (`parent.UserConstructionScript`))